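; BP_PSL_Demo is a demo Blueprint that receives heart rate readings over MQTT from a broker on localhost.
; On BeginPlay it creates and connects an MQTT client, then subscribes to the psl/hr topic without waiting for the connect callback, which only prints a success message.
; Its message handler parses each payload as JSON and stores the hr field in the HeartRate variable.
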(event `self.ReceiveBeginPlay`
  (bind _returnvalue (`MqttUtilitiesBPL.CreateMqttClient` (make `MqttClientConfig` "127.0.0.1" 1883 "UEClient_01" 100)))
  (`MqttClientInterface.Connect` _returnvalue (make `MqttConnectionData` "") (delegate `OnConnect_new`))
  (message `MqttClientInterface.Subscribe` (`KismetSystemLibrary.Conv_InterfaceToObject` _returnvalue) "psl/hr" 0)
  (`MqttClientInterface.SetOnMessageHandler` _returnvalue (delegate `CustomEvent`)))

(event `CustomEvent`
  (params (message :type "MqttMessage Structure"))
  (bind _outjsonobject (`JsonBlueprintFunctionLibrary.FromString` (`.Message` (break `MqttMessage` message))))
  (bind _outvalue (`|GetJsonField` _outjsonobject "hr"))
  (set `self.HeartRate` _outvalue))

(event `OnConnect_new`
  (`KismetSystemLibrary.PrintString` "Chris: Connected to MQTT Client Successfully"))

(fn `UserConstructionScript`)